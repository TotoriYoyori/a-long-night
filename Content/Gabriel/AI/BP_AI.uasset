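; BP_AI is an AI-controlled pawn that reacts to sensed pawns and plays voice and footstep sounds.
; PawnSensing sight and hearing events latch flags into blackboard keys, with no player check and no reset; only sight updates followPlayer.
; Sighting also plays a random attached sound, gated by a short cooldown.
; A looping timer plays footstep sounds whenever the pawn has velocity.
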(event `self.PawnSensing.OnSeePawn`
  (params (Pawn :type "Pawn Object Reference"))
  (if true
    (`BlackboardComponent.SetValueAsBool` (`AIBlueprintHelperLibrary.GetBlackboard` (`AIBlueprintHelperLibrary.GetAIController` self)) "seeingPlayer" true)
    (bind _output_get (set `self.playerSeen` true))
    (`BlackboardComponent.SetValueAsBool` (`AIBlueprintHelperLibrary.GetBlackboard` (`AIBlueprintHelperLibrary.GetAIController` self)) "followPlayer" (or _output_get (stale `self.PawnSensing.OnHearNoise` _output_get)))
    (if (not (`self.SoundPlayed`))
      (set `self.SoundPlayed` true)
      (`GameplayStatics.SpawnSoundAttached` (`KismetArrayLibrary.Array_Random` (`self.SoundArray`)) (`self.Audio`) "None" (0.0 0.0 0.0) (struct) "KeepRelativeOffset" false 1.0 1.0 0.0 null null)
      (`KismetSystemLibrary.Delay` 5.0)
      (set `self.SoundPlayed` false))))

(event `self.PawnSensing.OnHearNoise`
  (params (Instigator :type "Pawn Object Reference") (Location :type "Vector Structure (by ref)") (Volume :type "Float (single-precision)"))
  (if true
    (`BlackboardComponent.SetValueAsBool` (`AIBlueprintHelperLibrary.GetBlackboard` (`AIBlueprintHelperLibrary.GetAIController` self)) "hearingPlayer" true)
    (bind _output_get (set `self.playerHeard` true))))

(event `self.ReceiveBeginPlay`
  (`KismetSystemLibrary.K2_SetTimerDelegate` (delegate `Play Footsteps Sounds`) 1.5 true))

(event `Play Footsteps Sounds`
  (`/Engine/EditorBlueprintResources/StandardMacros.CompareFloat` (`KismetMathLibrary.VSize` (`self.GetVelocity` self))
    (:`>`
      (`GameplayStatics.SpawnSoundAttached` "/Game/Gabriel/Wendigo_Sounds/FootstepsSound.FootstepsSound" (`self.Audio`) "None" (0.0 0.0 0.0) (struct) "KeepRelativeOffset" false 1.0 1.0 0.0 null null))))

(fn `UserConstructionScript`)